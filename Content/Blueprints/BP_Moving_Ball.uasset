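; Moving ball actor that bounces off blocking surfaces, apparently for a paddle-and-ball game.
; BeginPlay takes the initial direction from the ball to a pointer component, without normalizing it.
; Tick moves the actor with a swept offset scaled by Velocity, reflecting direction off hit normals with Z zeroed.
; Overlapping a KillZVolume calls BallDestroyed and destroys the actor; the player-platform Hit handler only casts, with no further action.
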(event `self.ReceiveBeginPlay`
  ;[1 1 1] Направляет ветор движения в сторону указателя
  (set `self.Direction` (- (`SceneComponent.K2_GetComponentLocation` (`self.Base_Direction_Pointer`)) (`SceneComponent.K2_GetComponentLocation` (`self.Ball`)))))

(event `self.ReceiveActorBeginOverlap`
  (params (OtherActor :type "Actor Object Reference"))
  (cast `KillZVolume` OtherActor)
  (`self.Ball_Destroyed`)
  (`self.K2_DestroyActor`))

(event `self.ReceiveTick`
  (params (DeltaSeconds :type "Float (single-precision)"))
  ;[1 1 1] Движение шарика с отражением
  (bind _sweephitresult (`self.K2_AddActorWorldOffset` (* (* (`self.Direction`) (`self.Velocity`)) DeltaSeconds) true))
  (bind (_bblockinghit _binitialoverlap _time _distance _location _impactpoint _normal) (`GameplayStatics.BreakHitResult` _sweephitresult))
  (if _bblockinghit
    (bind (_returnvalue_x _returnvalue_y) (`KismetMathLibrary.BreakVector` (`KismetMathLibrary.GetReflectionVector` (`self.Direction`) _normal)))
    (set `self.Direction` (`KismetMathLibrary.MakeVector` _returnvalue_x _returnvalue_y))))

(event `self.ReceiveHit`
  (params (MyComp :type "PrimitiveComponent Object Reference") (Other :type "Actor Object Reference") (OtherComp :type "PrimitiveComponent Object Reference") (bSelfMoved :type Boolean) (HitLocation :type "Vector Structure") (HitNormal :type "Vector Structure") (NormalImpulse :type "Vector Structure") (Hit :type "HitResult Structure (by ref)"))
  (cast `/Game/Blueprints/BP_Player_Platform` Other))

(fn `UserConstructionScript`)